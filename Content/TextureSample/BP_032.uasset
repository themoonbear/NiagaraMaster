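; Sample Blueprint that cycles logo textures shown by a Niagara particle effect.
; On BeginPlay it enables input from player controller 0.
; Each press of D advances an index that wraps through LOGOList, sets that texture on the Niagara User.LOGO parameter and reinitializes the system.
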(event EventBeginPlay
  (Input|EnableInput (Game|GetPlayerController 0)))

(event Input|KeyboardEvents|D
  (params (Key :type Key%20Structure :default "None"))
  (bind _niagara (Variables|Default|GetNiagara))
  (bind _logolist (Variables|Default|GetLOGOList))
  (bind _logoindex (Variables|Default|GetLogoIndex))
  (:Pressed
    (Math|Integer|IncrementInt _logoindex
      (:%20%20
        (Niagara|SetTextureObject _niagara "User.LOGO" (Utilities|Array|Get(acopy) _logolist (Math|Integer|%(Integer) _logoindex (Utilities|Array|Length _logolist))))
        (Niagara|ReinitializeSystem _niagara)))))

(fn ConstructionScript)