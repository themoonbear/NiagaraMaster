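; BP_03 is a texture sample actor that cycles the texture shown by its Niagara effect when the H key is pressed.
; It enables input from player controller 0 on BeginPlay.
; Each press increments an index, wraps it over a texture list, sets that texture on the Niagara User.LOGO parameter and reinitializes the system to apply it.
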(event EventBeginPlay
  (Input|EnableInput (Game|GetPlayerController 0)))

(event Input|KeyboardEvents|H
  (params (Key :type Key%20Structure :default "None"))
  (bind _niagara (Variables|Default|GetNiagara))
  (bind _texture_index (Variables|Default|GetTexture_Index))
  (bind _texturelist (Variables|Default|GetTextureList))
  (:Pressed
    (Math|Integer|IncrementInt _texture_index
      (:%20%20
        (Niagara|SetTextureObject _niagara "User.LOGO" (Utilities|Array|Get(acopy) _texturelist (Math|Integer|%(Integer) _texture_index (Utilities|Array|Length _texturelist))))
        (Niagara|ReinitializeSystem _niagara)))))

(fn ConstructionScript)