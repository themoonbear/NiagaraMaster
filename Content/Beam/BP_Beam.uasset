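; BP_Beam is an input-driven actor that extends and retracts a Niagara beam effect.
; On BeginPlay it enables input from player controller 0, so holding B plays the VectorLerp timeline and releasing it reverses the timeline.
; Each timeline update lerps from the Niagara component's world location to the Arrow's and writes the result to the User.MyBeamEnd parameter, moving the beam's end point.
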(event EventBeginPlay
  (Input|EnableInput (Game|GetPlayerController 0)))

(event Input|KeyboardEvents|B
  (params (Key :type Key%20Structure :default "None"))
  (:Pressed
    (bind _verctorlerp (Timeline|VectorLerp Play)
      (:Update
        (Niagara|SetNiagaraVariable(Vector3) (Variables|Default|GetNiagara) "User.MyBeamEnd" (Math|Vector|Lerp(Vector) (Transformation|GetWorldLocation (Variables|Default|GetNiagara)) (Transformation|GetWorldLocation (Variables|Default|GetArrow)) _verctorlerp)))))
  (:Released
    (Timeline|VectorLerp Reverse)))

(fn ConstructionScript)